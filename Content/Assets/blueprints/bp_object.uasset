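; Grabbable physics object for a goal task: it must stay at a Bp_destination to complete the goal.
; PickUp attaches it with physics off, and DropOff detaches it and restores physics.
; GoalReached plays a found cue and re-triggers itself by timer; the second pass destroys the object and fires GoalCompleted.
; Leaving the destination resets count, timer and sound, while the Bp_button's red-button click destroys the object.
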(event Custom|redButtonClicked
  (Actor|DestroyActor))

(event Custom|goalReached
  (bind _returnvalue (Utilities|Time|SetTimerbyEvent (delegate Custom|goalReached) 4.3))
  (Transformation|SetWorldLocation (Variables|Default|GethideNseek-objectFound_Cue) (Transformation|GetWorldLocation (Variables|Default|Getobject_mesh)) false false)
  (Audio|Components|Audio|Play (Variables|Default|GethideNseek-objectFound_Cue) 0.0)
  (bind _result (Math|Integer|IncrementInt (Variables|Default|GetgoalTime))
    (:%20%20
      (bind _output_get (Variables|Default|SetgoalTime _result))
      (if (>= _output_get 2)
        (Actor|DestroyActor)
        (Default|CallGoalCompleted)))))

(event EventBeginPlay
  (Audio|Components|Audio|Stop (Variables|Default|GethideNseek-objectFound_Cue))
  (bind _outactors (Actor|GetAllActorsOfClass "/Game/Assets/blueprints/bp_button.bp_button_C"))
  (bind _output_get (Variables|Default|SetbuttonRestart (Utilities|Array|Get(acopy) _outactors)))
  (EventDispatchers|BindEventtoRedButtonClicked _output_get (delegate Custom|redButtonClicked)))

(event EventDropOff
  (Physics|SetSimulatePhysics (Variables|Default|Getobject_mesh) true)
  (Transformation|DetachFromActor "KeepWorld" "KeepWorld" "KeepWorld"))

(event Collision|EventActorEndOverlap
  (params (OtherActor :type Actor%20Object%20Reference))
  (if (== (Utilities|GetClass OtherActor) "/Game/Assets/blueprints/bp_destination.bp_destination_C")
    (Variables|Default|SetgoalTime 0)
    (Utilities|Time|ClearandInvalidateTimerbyHandle (stale Custom|goalReached _returnvalue))
    (Audio|Components|Audio|Stop (Variables|Default|GethideNseek-objectFound_Cue))))

(event EventPickUp
  (params (ActorToAttachTo :type Scene%20Component%20Object%20Reference))
  (Physics|SetSimulatePhysics (Variables|Default|Getobject_mesh) false)
  (Transformation|AttachComponentToComponent (VehicleSound|GetRootComponent) ActorToAttachTo "None" "KeepWorld" "KeepWorld" "KeepWorld" true))

(fn ConstructionScript)