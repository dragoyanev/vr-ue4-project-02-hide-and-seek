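; BP_Button is a pressable button for VR that fires a RedButtonClicked call when the player's VR pawn touches it.
; Begin overlap on the button mesh checks for the exact Bp_MyVRPawn class, makes the call and plays the Animation timeline.
; The timeline lerps the mesh's relative scale between starting and ending values.
; End overlap by any actor reverses the timeline.
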(event OnComponentBeginOverlap(botton_mesh)
  (params (OverlappedComponent :type Primitive%20Component%20Object%20Reference) (OtherActor :type Actor%20Object%20Reference) (OtherComp :type Primitive%20Component%20Object%20Reference) (OtherBodyIndex :type Integer) (bFromSweep :type Boolean) (SweepResult :type Hit%20Result%20Structure%20%28by%20ref%29))
  (if (== (Utilities|GetClass OtherActor) "/Game/Assets/player/bp_MyVRPawn.bp_MyVRPawn_C")
    (Default|CallRedButtonClicked)
    (bind _alpha (Timeline|animation Play)
      (:Update
        (Transformation|SetRelativeScale3D (Variables|Default|Getbotton_mesh) (Math|Vector|Lerp(Vector) (Variables|Default|GetstartingScale) (Variables|Default|GetendingScale) _alpha))))))

(event OnComponentEndOverlap(botton_mesh)
  (params (OverlappedComponent :type Primitive%20Component%20Object%20Reference) (OtherActor :type Actor%20Object%20Reference) (OtherComp :type Primitive%20Component%20Object%20Reference) (OtherBodyIndex :type Integer))
  (bind _alpha (Timeline|animation Reverse)
    (:Update
      (Transformation|SetRelativeScale3D (Variables|Default|Getbotton_mesh) (Math|Vector|Lerp(Vector) (Variables|Default|GetstartingScale) (Variables|Default|GetendingScale) _alpha)))))

(fn ConstructionScript)